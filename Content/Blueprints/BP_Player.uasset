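; Player Blueprint for a networked game, showing local net role, rocket count and health on a WBP_Role widget.
; BeginPlay caches the widget and adds an FGValueReplicator named SmoothValue, whose value Tick prints each frame and the B key raises by a random amount.
; The authority picks a random Color at BeginPlay, which OnRep_Color applies to the materials.
; Rocket and health change events update the widget.
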(event EventBeginPlay
  (bind _returnvalue (Class|FGReplicatorComponent|AddReplicatorbyClass (Variables|Default|GetFGReplicator) "/Script/FGNet.FGValueReplicator" "SmoothValue"))
  (bind _asfgvalue_replicator (Utilities|Casting|CastToFGValueReplicator _returnvalue))
  (Variables|Default|SetValueReplicator _asfgvalue_replicator)
  (bind _aswbp_role (Utilities|Casting|CastToWBP_Role (UserInterface|GetUserWidgetObject (Variables|Default|GetWidget_Role))))
  (bind _output_get (Variables|Default|SetRef_WBP_Role _aswbp_role))
  (CallFunction|SetLocalText _output_get)
  (Networking|SwitchHasAuthority
    (:Authority
      (Variables|Default|SetColor (Utilities|Struct|MakeLinearColor (Math|Random|RandomFloatinRange 0.0 1.0) (Math|Random|RandomFloatinRange 0.0 1.0) (Math|Random|RandomFloatinRange 0.0 1.0) 1.0)))))

(event EventOnNumRocketsChanged
  (params (NewNumrockets :type Integer))
  (bind _ref_wbp_role (Variables|Default|GetRef_WBP_Role)
    (:then
      (CallFunction|SetNumRocketsinWidget _ref_wbp_role NewNumrockets))
    (:else)))

(event EventOnHealthChanged
  (params (CurrentHealth :type Float%20%28single-precision%29))
  (bind _ref_wbp_role (Variables|Default|GetRef_WBP_Role)
    (:then
      (Default|SetHealthTextandBar _ref_wbp_role CurrentHealth))
    (:else)))

(event EventTick
  (params (DeltaSeconds :type Float%20%28single-precision%29))
  (Development|PrintString (Utilities|String|ToString(Float) (Class|FGValueReplicator|GetValue (Variables|Default|GetValueReplicator))) true false "(R=0.000000,G=0.660000,B=1.000000,A=1.000000)" DeltaSeconds))

(event Input|KeyboardEvents|B
  (params (Key :type Key%20Structure :default "None"))
  (bind _valuereplicator (Variables|Default|GetValueReplicator))
  (:Pressed
    (Class|FGValueReplicator|SetValue _valuereplicator (+ (Class|FGValueReplicator|GetValue _valuereplicator) (Math|Random|RandomFloatinRange 1e+01 2e+02)))))

(fn ConstructionScript)

(fn SetLocalText
  (params (WBP_Role :type WBP%20Role%20Object%20Reference))
  (Default|SetLocalText WBP_Role (Utilities|Text|ToText(String) (Utilities|String|EnumtoString (Networking|GetLocalRole)))))

(fn SetNumRocketsinWidget
  (params (WBP_Role :type WBP%20Role%20Object%20Reference) (InNumRockets :type Integer))
  (Default|SetNumRockets WBP_Role InNumRockets))

(fn OnRepColor
  (Class|FGPlayer|ChangeMaterialColors (Math|Conversions|ToColor(LinearColor) (Variables|Default|GetColor))))